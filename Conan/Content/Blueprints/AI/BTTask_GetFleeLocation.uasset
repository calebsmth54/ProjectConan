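; Behavior Tree task that picks a navigable location for an AI to flee from the actor in FleeFromKey.
; It projects FleeDistance plus FleeRadius along the flattened direction away from that actor, then stores a random reachable point within FleeRadius there in FleeTargetKey.
; It draws debug shapes and fails when no point is found.
; An invalid FleeFromKey actor only prints a warning, without calling FinishExecute.
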(event EventReceiveExecute
  (params (OwnerActor :type Actor%20Object%20Reference))
  (bind _returnvalue (Transformation|GetActorLocation OwnerActor))
  (bind _returnvalue_2 (Transformation|GetActorLocation OwnerActor))
  (bind _fleefromkey (Variables|Default|GetFleeFromKey))
  (bind _fleedistance (Variables|Default|GetFleeDistance))
  (bind _fleeradius (Variables|Default|GetFleeRadius))
  (bind _fleeradius_2 (Variables|Default|GetFleeRadius))
  (bind _returnvalue_3 (AI|BehaviorTree|GetBlackboardValueasActor _fleefromkey))
  (bind _returnvalue_4 (+ _fleedistance _fleeradius_2))
  (bind _returnvalue_5 (Transformation|GetActorLocation _returnvalue_3))
  (bind _returnvalue_6 (- (Math|Vector|MakeVector (.x _returnvalue_5) (.y _returnvalue_5) 0.0) (Math|Vector|MakeVector (.x _returnvalue_2) (.y _returnvalue_2) 0.0)))
  (bind _returnvalue_7 (* _returnvalue_6 -1.0))
  (bind _returnvalue_8 (Math|Vector|MakeVector (.x _returnvalue_7) (.y _returnvalue_7) 0.0))
  (bind _returnvalue_9 (Math|Vector|Normalize _returnvalue_8))
  (bind _returnvalue_10 (* _returnvalue_9 _returnvalue_4))
  (bind _returnvalue_11 (+ _returnvalue _returnvalue_10))
  (bind (_randomlocation _returnvalue_12) (AI|Navigation|GetRandomReachablePointinRadius _returnvalue_11 _fleeradius))
  (Class|BTFunctionLibrary|ClearBlackboardValue (Variables|Default|GetFleeTargetKey))
  (Utilities|IsValid _returnvalue_3
    (:Is%20Valid
      ;[1 1 1] Debug
      (Rendering|Debug|DrawDebugLine _returnvalue _returnvalue_11 "(R=0.937500,G=0.194809,B=0.185483,A=1.000000)" 5.0 5.0)
      (Rendering|Debug|DrawDebugSphere _returnvalue_11 (Variables|Default|GetFleeRadius) 12 "(R=1.000000,G=0.000000,B=0.015782,A=1.000000)" 5.0 5.0)
      (if _returnvalue_12
        (AI|BehaviorTree|SetBlackboardValueasVector (Variables|Default|GetFleeTargetKey) _randomlocation)
        (Rendering|Debug|DrawDebugPoint _randomlocation 5.0 "(R=0.844961,G=0.109964,B=0.885417,A=1.000000)" 5.0)
        (AI|BehaviorTree|FinishExecute true)
        (else
          ;[1 1 1] Failed! Start cowering
          (AI|BehaviorTree|FinishExecute false))))
    (:Is%20Not%20Valid
      (Development|PrintString "FleeFromKey not set to an actor!" true true "(R=1.000000,G=0.211646,B=0.071805,A=1.000000)"))))
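; Player vampire character with lurk/sprint movement, selectable powers, a blood tank and a feeding "embrace".
; Lurk and sprint toggle crouch and drive a Wwise RTPC; powers are gathered from attached PowerComp components.
; An overlap sphere tracks blood bags, scored by camera-direction dot product over squared distance.
; Embrace halts the target's AI, moves the player in, then starts timed draining; sucked blood feeds HealthComp, whose return value fills the tank.
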(event OnComponentBeginOverlap(EmbraceSphere)
  (params (OverlappedComponent :type Primitive%20Component%20Object%20Reference) (OtherActor :type Actor%20Object%20Reference) (OtherComp :type Primitive%20Component%20Object%20Reference) (OtherBodyIndex :type Integer) (bFromSweep :type Boolean) (SweepResult :type Hit%20Result%20Structure%20%28by%20ref%29))
  (bind _returnvalue (Actor|GetComponentbyClass OtherActor "/Game/Blueprints/Components/BloodBagComp.BloodBagComp_C"))
  ;[1 1 1] Find tasty blood bags
  (if (!= OtherActor self)
    (Utilities|IsValid _returnvalue
      (:Is%20Valid
        (Utilities|Array|AddUnique (Variables|Embrace|GetNearByBloodBags) _returnvalue)
        (Development|PrintString (Utilities|String|Append "A new blood bag has appeared nearby: " (Utilities|GetDisplayName (Components|GetOwner _returnvalue))))))))

(event OnComponentEndOverlap(EmbraceSphere)
  (params (OverlappedComponent :type Primitive%20Component%20Object%20Reference) (OtherActor :type Actor%20Object%20Reference) (OtherComp :type Primitive%20Component%20Object%20Reference) (OtherBodyIndex :type Integer))
  (bind _returnvalue (Actor|GetComponentbyClass OtherActor "/Game/Blueprints/Components/BloodBagComp.BloodBagComp_C"))
  ;[1 1 1] Find tasty blood bags
  (Utilities|IsValid _returnvalue
    (:Is%20Valid
      (Utilities|Array|RemoveItem (Variables|Embrace|GetNearByBloodBags) _returnvalue))))

(event Custom|OnDeath
  ;[1 1 1] Handle Death
)

(event EventBeginPlay
  (bind _charactermovement (Variables|Character|GetCharacterMovement))
  ;[1 0.7928 0.2557] Begin Play
  ;;[1 1 1] Use our lurking speed for the walk speed
  (Variables|/Script/Engine.CharacterMovementComponent|SetMaxWalkSpeedCrouched _charactermovement (Variables|Movement|GetLurkSpeed))
  (Variables|/Script/Engine.CharacterMovementComponent|SetMaxWalkSpeed _charactermovement (Variables|Movement|GetSprintSpeed))
  (Movement|OnBeginLurk)
  ;;[1 1 1] Handle Death
  (EventDispatchers|BindEventtoOnNoHealth (Variables|Components|GetHealthComp) (delegate Custom|OnDeath))
  (BloodTanks|InitializeBloodTanks)
  (Powers|InitializePowers)
  ;;[1 1 1] Do this at the end because we need to initialize things here first
  (bind _asplayer_vamp_controller (Utilities|Casting|CastToPlayerVampController (Pawn|GetController)))
  (Default|InitHud _asplayer_vamp_controller))

(fn ConstructionScript)

(fn OnBeginLurk
  (Class|AkGameplayStatics|SetRTPCValue "ShadeRunCrouch" 0.0 1000 (Components|GetOwner))
  (if (not (Variables|Embrace|GetIsEmbracing?))
    (Character|Crouch)))

(fn OnBeginSprint
  (Class|AkGameplayStatics|SetRTPCValue "ShadeRunCrouch" 1e+02 1000 (Components|GetOwner))
  (if (not (Variables|Embrace|GetIsEmbracing?))
    (Character|UnCrouch)))

(fn UsePower
  (bind _powersinstances (Variables|Powers|GetPowersInstances))
  (bind _selectedpower (Variables|Powers|GetSelectedPower))
  (if (Utilities|Array|IsValidIndex _powersinstances _selectedpower)
    (Default|UsePower (Utilities|Array|Get(acopy) _powersinstances _selectedpower))
    (else
      (Development|PrintString "Invalid power!" true true "(R=1.000000,G=0.038692,B=0.000000,A=1.000000)"))))

(fn InitializeBloodTanks
  (Variables|BloodTanks|SetBloodTankAmount (Math|Conversions|ToFloat(Integer) (Variables|BloodTanks|GetNumOfBloodTanks))))

(fn CanUseBlood?
  (params (Amount :type Float%20%28single-precision%29))
  (if (>= (- (Variables|BloodTanks|GetBloodTankAmount) Amount) 0.0) ; Is there enough blood available?
    (return true)
    (else
      (return false))))

(fn UseBlood
  (params (Amount :type Float%20%28single-precision%29))
  (Variables|BloodTanks|SetBloodTankAmount (- (Variables|BloodTanks|GetBloodTankAmount) Amount))
  (return))

(fn InitializePowers
  (bind _returnvalue (Actor|GetComponentsByClass "/Game/Blueprints/Player/Powers/PowerComp.PowerComp_C"))
  (for _index (range 0 (- (Utilities|Array|Length _returnvalue) 1))
    (Utilities|Array|Add (Variables|Powers|GetPowersInstances) (Utilities|Array|Get(acopy) _returnvalue _index))))

(fn GetNumOfPowers
  (return (Utilities|Array|Length (Variables|Powers|GetPowersInstances))))

(fn FindNearestBloodBag
  (bind _nearbybloodbags (Variables|Embrace|GetNearByBloodBags))
  (for (_array_element _array_index) (Variables|Embrace|GetNearByBloodBags)
    ;[1 1 1] Compare score to highest value
    (if (> (* (Math|Vector|DotProduct (.Direction (Aim|GetAimLocationandDirection)) (Math|Vector|Normalize (- (Transformation|GetActorLocation) (Transformation|GetActorLocation (Components|GetOwner _array_element))))) (/ 1.0 (Math|Vector|VectorLengthSquared (- (Transformation|GetActorLocation) (Transformation|GetActorLocation (Components|GetOwner _array_element)))))) (LocalVariables|GetHighestBloodBagScore))
      (bind _output_get (LocalVariables|SetBestBloodBagIndex _array_index))
      (Development|PrintString (Utilities|String|Append "New blood bag score: " (Utilities|String|ToString(Integer) _output_get)))))
  (if (Utilities|Array|IsValidIndex _nearbybloodbags (LocalVariables|GetBestBloodBagIndex))
    (return (Utilities|Array|Get(acopy) _nearbybloodbags (LocalVariables|GetBestBloodBagIndex)) (Components|GetOwner (Utilities|Array|Get(acopy) _nearbybloodbags (LocalVariables|GetBestBloodBagIndex))))
    (else
      (Development|PrintString "No valid blood bags in the vicinity!" true true "(R=1.000000,G=0.000000,B=0.064642,A=1.000000)")
      (return 0 0))))

(fn AttemptEmbrace
  (if (not (Variables|Embrace|GetIsEmbracing?))
    (bind (_bestbloodbag _owner) (Embrace|FindNearestBloodBag))
    (Utilities|IsValid _bestbloodbag
      (:Is%20Valid
        (Embrace|OnStartEmbrace _bestbloodbag _owner))
      (:Is%20Not%20Valid
        (Embrace|OnEmbraceFailed)))))

(fn OnEmbraceFailed)

(fn OnStartEmbrace
  (params (BloodBag :type Blood%20Bag%20Comp%20Object%20Reference) (Owner :type Actor%20Object%20Reference))
  (bind _returnvalue (Game|GetPlayerController 0))
  (Variables|Embrace|SetIsEmbracing? true)
  (bind _ascharacter (Utilities|Casting|CastToCharacter Owner))
  ;[1 1 1] Stop AI Target
  (AI|Navigation|StopMovement (AI|GetAIController _ascharacter))
  (AI|Logic|StopLogic (Variables|/Script/AIModule.AIController|GetBrainComponent (AI|GetAIController _ascharacter)) "They're getting fed on yo!")
  ;[1 1 1] Disable our input and move us toward our target
  (AI|Navigation|StopMovement _returnvalue)
  (Input|SetIgnoreMoveInput _returnvalue true)
  (AI|Navigation|SimpleMovetoActor _returnvalue Owner)
  (Variables|Embrace|SetEmbraceBloodBag BloodBag)
  (Variables|Embrace|SetEmbraceOwner Owner)
  (Utilities|Time|SetTimerbyFunctionName self "OnEmbraceMoveFinished" (Variables|Embrace|GetEmbraceMoveWaitTime)))

(fn OnEmbraceMoveFinished
  (Default|BeginDraining (Variables|Embrace|GetEmbraceBloodBag) self (Pawn|GetController) (Variables|Embrace|GetEmbraceLength)))

(fn OnSuckBlood
  (params (BloodAmount :type Float%20%28single-precision%29%20%28by%20ref%29))
  (bind _healthoverflow (Default|GiveHealth (Variables|Components|GetHealthComp) BloodAmount))
  (BloodTanks|GiveBloodtoTank _healthoverflow)
  (Development|PrintString "Gulp Gulp"))

(fn OnEmbraceFinished
  (Variables|Embrace|SetIsEmbracing? false)
  (Input|SetIgnoreMoveInput (Game|GetPlayerController 0) false))

(fn GiveBloodtoTank
  (params (Amount :type Float%20%28single-precision%29))
  (Variables|BloodTanks|SetBloodTankAmount (Math|Float|Min(Float) (Math|Conversions|ToFloat(Integer) (Variables|BloodTanks|GetNumOfBloodTanks)) (+ Amount (Variables|BloodTanks|GetBloodTankAmount)))))

(fn GetAimLocationandDirection
  (bind _followcamera (Variables|Components|GetFollowCamera))
  (return (Transformation|GetWorldLocation _followcamera) (Math|Vector|GetForwardVector _followcamera)))
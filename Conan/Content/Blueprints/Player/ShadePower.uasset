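; ShadePower is a player power Blueprint that turns the vampire into a shade by hiding its mesh.
; PerformPower hides the VampRef mesh and its child components, then returns the parent's result.
; StopPower runs the parent logic, then unhides the mesh without propagating to children, so this Blueprint leaves those children hidden.
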(event EventBeginPlay
  (|CallParentFunction) ; This node is disabled and will not be called.\nDrag off pins to build functionality.
)

(event EventStopPower
  (|CallParentFunction)
  (CallFunction|TurntoReal))

(fn PerformPower
  (CallFunction|TurntoShade)
  (bind _success (|CallParentFunction))
  (return _success))

(fn TurntoReal
  (Development|SetHiddeninGame (Variables|/Script/Engine.Character|GetMesh (Variables|Default|GetVampRef)) false false))

(fn TurntoShade
  (Development|SetHiddeninGame (Variables|/Script/Engine.Character|GetMesh (Variables|Default|GetVampRef)) true true))
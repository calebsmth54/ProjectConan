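; Base-style power component for the vampire character that spends blood to activate a power.
; UsePower toggles the power: if VampCharacter has enough blood, it optionally drains instantly, starts a looping drain timer and calls PerformPower.
; PerformPower stops the power immediately unless DrainOverTime is set.
; Each timer tick drains blood again, stopping the power and clearing the timer when blood runs short.
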(event EventBeginPlay
  (bind _asvamp_character (Utilities|Casting|CastToVampCharacter (Components|GetOwner)))
  (Variables|Default|SetVampRef _asvamp_character))

(fn CanUsePower
  (return (Default|CanUseBlood? (Variables|Default|GetVampRef) (Variables|Default|GetDrainAmount))))

(fn UsePower
  ;[1 1 1] Toggle Timer if active
  (if (Variables|Default|GetActive?)
    (CallFunction|StopPower)
    (elif (CallFunction|CanUsePower)
      ;[1 1 1] Instantly drain
      (if (Variables|Default|GetInstantDrain?)
        (Default|UseBlood (Variables|Default|GetVampRef) (Variables|Default|GetDrainAmount)))
      (Variables|Default|SetActive? true)
      (CallFunction|StartTimerDrain)
      (bind _success (CallFunction|PerformPower))
      (return _success)
      (else
        (return false)))))

(fn PerformPower
  (if (not (Variables|Default|GetDrainOverTime?))
    (CallFunction|StopPower))
  (return true))

(fn OnTimerDrain
  (if (CallFunction|CanUsePower)
    (Default|UseBlood (Variables|Default|GetVampRef) (Variables|Default|GetDrainAmount))
    (else
      (CallFunction|StopPower))))

(fn StopPower
  (Variables|Default|SetActive? false)
  (Utilities|Time|ClearandInvalidateTimerbyHandle (Variables|Default|GetDrainTimer)))

(fn StartTimerDrain
  (bind _returnvalue (Utilities|Time|SetTimerbyFunctionName 0 (Variables|Default|GetOnTimerDrainString) (Variables|Default|GetDrainTime) true))
  (Variables|Default|SetDrainTimer _returnvalue))
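; TeleportPower is an unfinished player power Blueprint for a vampire character, built on a parent power class.
; CanUsePower line traces from the character toward the scaled controller forward vector, not offset by its location, then capsule traces at the hit using the character's capsule size.
; Both traces draw debug shapes, but their results never decide the outcome, which is always false.
; PerformPower only calls the parent, so no teleport happens here.
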(event EventBeginPlay
  (|CallParentFunction) ; This node is disabled and will not be called.\nDrag off pins to build functionality.
)

(event EventTick
  (params (DeltaSeconds :type Float%20%28single-precision%29)))

(fn PerformPower
  (bind _success (|CallParentFunction))
  (return _success))

(fn CanUsePower
  (bind _vampref (Variables|Default|GetVampRef))
  (bind _vampref_2 (Variables|Default|GetVampRef))
  (bind _capsulecomponent (Variables|/Script/Engine.Character|GetCapsuleComponent _vampref))
  (bind (_outradius _outhalfheight) (Components|Capsule|GetScaledCapsuleSize _capsulecomponent))
  (if (|CallParentFunction)
    (bind _outhit (Collision|LineTraceByChannel (Transformation|GetActorLocation _vampref_2) (* (Transformation|GetActorForwardVector (Pawn|GetController _vampref_2)) (Variables|Default|GetTeleportDistance)) "TraceTypeQuery1" false 0 "ForDuration"))
    (Collision|CapsuleTraceByChannel (.location _outhit) (.location _outhit) _outradius _outhalfheight "TraceTypeQuery1" true 0 "ForDuration")
    (return false)
    (else
      (return false))))
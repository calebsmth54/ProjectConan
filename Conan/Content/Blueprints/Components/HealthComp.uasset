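; HealthComp is an actor component that tracks its owner's health and handles reaching zero.
; On BeginPlay it fills health from a starting value and binds to the owner's OnTakeAnyDamage to subtract incoming damage.
; At or below zero it broadcasts OnNoHealth, then ragdolls Character owners through mesh physics and collision.
; Getters expose current health and its fraction of the starting value; health is not clamped.
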(event Custom|TakeDamage
  (params (DamagedActor :type Actor%20Object%20Reference) (Damage :type Float%20%28single-precision%29) (DamageType :type Damage%20Type%20Object%20Reference) (InstigatedBy :type Controller%20Object%20Reference) (DamageCauser :type Actor%20Object%20Reference))
  ;[0.03963 0.2093 1] Handle Damage Taken
  (bind _output_get (Variables|Default|SetCurrentHealth (- (Variables|Default|GetCurrentHealth) Damage)))
  (if (<= _output_get 0.0)
    (Default|CallOnNoHealth) ; Notify our listeners
    ;;[1 1 1] Ragdoll characters
    (bind _ascharacter (Utilities|Casting|CastToCharacter (Components|GetOwner)))
    (Physics|SetSimulatePhysics (Variables|/Script/Engine.Character|GetMesh _ascharacter) true)
    (Collision|SetCollisionEnabled (Variables|/Script/Engine.Character|GetMesh _ascharacter) "QueryAndPhysics")))

(event EventBeginPlay
  ;[1 0.7589 0.5194] Event Begin Play
  (Variables|Default|SetCurrentHealth (Variables|Default|GetStartingHealth))
  (EventDispatchers|BindEventtoOnTakeAnyDamage (Components|GetOwner) (delegate Custom|TakeDamage)))

(fn GetHealth
  (return (Variables|Default|GetCurrentHealth)))

(fn GetHealthpercent
  (return (/ (Variables|Default|GetCurrentHealth) (Variables|Default|GetStartingHealth))))
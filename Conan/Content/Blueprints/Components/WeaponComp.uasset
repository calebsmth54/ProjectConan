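; Weapon component that handles fire-rate-limited automatic firing and broadcasts each shot through an OnFire event.
; Fire checks CanFire, fires immediately, then repeats through a looping FireTick timer.
; StopFiring swaps any pending loop for a one-shot DryFireTick of the remaining time, keeping IsFiring set until the cooldown ends so re-triggering cannot beat the fire rate.
; Tick prints the remaining timer time for debugging.
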(event EventTick
  (params (DeltaSeconds :type Float%20%28single-precision%29))
  (Development|PrintString (Utilities|String|Append "Fire Rate Timer: " (Utilities|String|ToString(Float) (Utilities|Time|GetTimerRemainingTimebyHandle (Variables|Default|GetFireRateTimer))))))

(fn Fire
  (if (CallFunction|CanFire?)
    (bind _returnvalue (Utilities|Time|SetTimerbyFunctionName self "FireTick" (Variables|Default|GetFireRate) true))
    (Variables|Default|SetFireRateTimer _returnvalue)
    (Variables|Default|SetIsFiring? true)
    (CallFunction|PerformFireAction)
    (return)))

(fn CanFire?
  (bind _fireratetimer (Variables|Default|GetFireRateTimer))
  (return (and (or (not (Utilities|Time|IsValidTimerHandle _fireratetimer)) (<= (Utilities|Time|GetTimerRemainingTimebyHandle _fireratetimer) 0.0)) (not (Variables|Default|GetIsFiring?)))))

(fn PerformFireAction
  (Default|CallOnFireEvent)
  (return true))

(fn StopFiring
  ;[1 1 1] Wait for the current attack to finish?
  (if (> (Utilities|Time|GetTimerRemainingTimebyHandle (Variables|Default|GetFireRateTimer)) 0.0)
    (bind _output_get (LocalVariables|SetTimeRemaining (Utilities|Time|GetTimerRemainingTimebyHandle (Variables|Default|GetFireRateTimer))))
    (Utilities|Time|ClearandInvalidateTimerbyHandle (Variables|Default|GetFireRateTimer))
    (bind _returnvalue (Utilities|Time|SetTimerbyFunctionName self "DryFireTick" _output_get))
    (Variables|Default|SetFireRateTimer _returnvalue)
    (return)
    (else
      (Utilities|Time|ClearandInvalidateTimerbyHandle (Variables|Default|GetFireRateTimer))
      (Variables|Default|SetIsFiring? false)
      (return))))

(fn DryFire
  (Variables|Default|SetIsFiring? false)
  (return true))

(fn FireTick
  (CallFunction|PerformFireAction))

(fn DryFireTick
  (CallFunction|DryFire)
  (return))
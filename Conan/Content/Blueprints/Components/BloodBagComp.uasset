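; Actor component that makes its owner a blood source a vampire can drain over a timed embrace.
; BeginDraining stores the vampire and controller, derives a per-tick amount from drain length divided by DrainRate, and starts looping tick and finish timers.
; Each tick lowers the bag's capacity and feeds the vampire that amount scaled by BagQuality.
; Finishing stops ticking, applies embrace damage to kill the owner, and notifies the vampire.
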(event EventBeginPlay
  (Variables|Default|SetCurrentBagCapacity (Variables|Default|GetBagCapacity)))

(fn BeginDraining
  (params (Vamp :type Vamp%20Character%20Object%20Reference) (VampController :type Controller%20Object%20Reference) (DrainLength :type Float%20%28single-precision%29))
  (Variables|Default|SetBloodsucker Vamp)
  (Variables|Default|SetBloodSuckerController VampController)
  ;[1 1 1] Calculate Drain Rate Amount
  (Variables|Default|SetDrainRateAmount (/ DrainLength (Variables|Default|GetDrainRate)))
  ;[1 1 1] Set timers for drain tick and finish drain
  (bind _returnvalue (Utilities|Time|SetTimerbyFunctionName self "OnFinishedDrain" DrainLength))
  (Variables|Default|SetDrainFinishTimer _returnvalue)
  (bind _returnvalue_2 (Utilities|Time|SetTimerbyFunctionName self "OnDrainTick" (Variables|Default|GetDrainRate) true))
  (Variables|Default|SetDrainTickTimer _returnvalue_2))

(fn OnDrainTick
  (Variables|Default|SetCurrentBagCapacity (- (Variables|Default|GetCurrentBagCapacity) (Variables|Default|GetDrainRateAmount)))
  ;[1 1 1] Feed our vampiric fiend
  (Default|OnSuckBlood (Variables|Default|GetBloodsucker) (* (Variables|Default|GetDrainRateAmount) (Variables|Default|GetBagQuality))))

(fn OnFinishedDrain
  (Utilities|Time|ClearandInvalidateTimerbyHandle (Variables|Default|GetDrainTickTimer))
  ;[1 1 1] Kill our owner
  (Game|Damage|ApplyDamage (Components|GetOwner) 1e+02 (Variables|Default|GetBloodSuckerController) (Variables|Default|GetBloodsucker) "/Game/Blueprints/Components/DamageType_EmbraceFinished.DamageType_EmbraceFinished_C")
  ;[1 1 1] Notify our bloodsucker that we are depleted...
  (Default|OnEmbraceFinished (Variables|Default|GetBloodsucker)))